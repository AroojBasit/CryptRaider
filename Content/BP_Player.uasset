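; BP_Player is the Crypt Raider player pawn, which grabs objects and wins the game by carrying the right item into an end zone.
; Grab input drives a Grabber component, and Escape quits the game.
; Capsule overlap with an EndTrigger-tagged actor sets a flag that Tick uses to keep checking the end condition.
; Holding an actor tagged Unlock2 then calls GameWon on the game mode, while any end overlap clears the flag.
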(event OnComponentBeginOverlap(CapsuleComponent)
  (params (OverlappedComponent :type Primitive%20Component%20Object%20Reference) (OtherActor :type Actor%20Object%20Reference) (OtherComp :type Primitive%20Component%20Object%20Reference) (OtherBodyIndex :type Integer) (bFromSweep :type Boolean) (SweepResult :type Hit%20Result%20Structure%20%28by%20ref%29))
  (if (Actor|ActorHasTag OtherActor "EndTrigger")
    (Variables|Default|SetEndTrigger true)
    (CallFunction|CheckEndCondition)))

(event Custom|CheckEndCondition
  (bind _grabber (Variables|Default|GetGrabber))
  (bind _returnvalue (Class|Grabber|GrabbedActor _grabber))
  (Utilities|IsValid _returnvalue
    (:Is%20Valid
      (if (Actor|ActorHasTag _returnvalue "Unlock2")
        (bind _asbp_crypt_raider_game_mode (Utilities|Casting|CastToBP_CryptRaiderGameMode (Game|GetGameMode)))
        (Default|GameWon _asbp_crypt_raider_game_mode)))))

(event EventBeginPlay)

(event Collision|EventActorBeginOverlap
  (params (OtherActor :type Actor%20Object%20Reference)))

(event EventTick
  (params (DeltaSeconds :type Float%20%28single-precision%29))
  (if (Variables|Default|GetEndTrigger)
    (CallFunction|CheckEndCondition)))

(event Collision|EventActorEndOverlap
  (params (OtherActor :type Actor%20Object%20Reference))
  (Variables|Default|SetEndTrigger false))

(event Input|ActionEvents|InputActionGrab
  (params (Key :type Key%20Structure :default "None"))
  (bind _grabber (Variables|Default|GetGrabber))
  (:Pressed
    (Class|Grabber|Grab _grabber))
  (:Released
    (Class|Grabber|Release _grabber)))

(event Input|KeyboardEvents|Escape
  (params (Key :type Key%20Structure :default "None"))
  (:Pressed
    (Game|QuitGame 0 "Quit" false)))

(event Input|KeyboardEvents|F
  (params (Key :type Key%20Structure :default "None")))

(fn ConstructionScript
  (|CallParentFunction))